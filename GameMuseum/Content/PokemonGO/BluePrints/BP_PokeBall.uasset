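; BP_PokeBall is a throwable Poké Ball that follows in front of the player until left mouse launches it to capture BP_Pikachu.
; A short delay loop repositions the ball and polls input; once thrown, Tick applies forward physics impulses every frame.
; Hitting Pikachu destroys it, the ball and ambient sounds, then plays the capture sound.
; Otherwise, after a one-second delay, the ball destroys itself and spawns a replacement.
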(event `self.ReceiveBeginPlay`
  ; Awake Method
  (`self.EnableInput` (`GameplayStatics.GetPlayerController` 0) null)
  (set `self.BallThorwed` false)
  (set `self.PikachuNotCatched` true)
  (bind _returnvalue (`|CreateWidget` "/Game/PokemonGO/InitialText.InitialText_C"))
  (bind _output_get (set `self.Text` _returnvalue))
  (`UserWidget.AddToViewport` _output_get 0)
  (`self.PBINPLayer`))

(event `self.ReceiveTick`
  (params (DeltaSeconds :type "Float (single-precision)"))
  ; Update Method (Called Every Frame)
  (if (and (`self.PikachuNotCatched`) (`self.BallThorwed`))
    (`self.AddBallImpulse`)
    (else
      (`self.K2_SetActorRotation` :`self` self))))

(event `PBINPLayer`
  (bind _returnvalue (`GameplayStatics.GetPlayerCharacter` 0))
  ; Move the Pokeball to the player's front
  (`self.K2_SetActorLocation` self (+ (* (`self.GetActorForwardVector` _returnvalue) (100.0 100.0 500.0)) (`self.K2_GetActorLocation` _returnvalue)) false false)
  (`self.ThrowBall`))

(event `ThrowBall`
  ; Throw Ball
  (if (`PlayerController.IsInputKeyDown` (`GameplayStatics.GetPlayerController` 0) "LeftMouseButton")
    (set `self.BallThorwed` true)
    (`GameplayStatics.PlaySound2D` "/Game/PokemonGO/Sound/ThrowBall.ThrowBall" 1.0 1.0 0.0 null null)
    (else
      (`KismetSystemLibrary.Delay` 0.001)
      (`self.PBINPLayer`))))

(event `AddBallImpulse`
  ; AddBall Impulse
  (`PrimitiveComponent.SetSimulatePhysics` (`self.PokeBall`) true)
  (`PrimitiveComponent.AddImpulse` (`self.PokeBall`) (* (`self.GetActorForwardVector` (`GameplayStatics.GetPlayerCharacter` 0)) (2000.0 2000.0 2000.0)) "None" false)
  (`KismetSystemLibrary.Delay` 1.0)
  (`self.CaptureFailed`))

(event `self.PokeBall.OnComponentHit`
  (params (HitComponent :type "PrimitiveComponent Object Reference") (OtherActor :type "Actor Object Reference") (OtherComp :type "PrimitiveComponent Object Reference") (NormalImpulse :type "Vector Structure") (Hit :type "HitResult Structure (by ref)"))
  ; Pikachu Catched
  (bind _asbp_pikachu (cast `/Game/PokemonGO/BluePrints/BP_Pikachu` OtherActor))
  (if (`self.BallThorwed`)
    (set `self.PikachuNotCatched` false)
    (set `self.BallThorwed` false)
    (`PrimitiveComponent.SetSimulatePhysics` (`self.PokeBall`) false)
    (bind _outactors (`GameplayStatics.GetAllActorsOfClass` "/Script/Engine.AmbientSound"))
    (`self.K2_DestroyActor` _outactors)
    (`self.K2_DestroyActor` _asbp_pikachu)
    (`GameplayStatics.PlaySound2D` "/Game/PokemonGO/Sound/Captured.Captured" 1.0 1.0 0.0 null null)
    (`self.K2_DestroyActor`)))

(event `CaptureFailed`
  (bind _returnvalue (`GameplayStatics.GetPlayerCharacter` 0))
  ; CaptureFailed
  (`PrimitiveComponent.SetSimulatePhysics` (`self.PokeBall`) false)
  (set `self.BallThorwed` false)
  (`self.K2_DestroyActor` self)
  (`|SpawnActorFromClass` "BP_PokeBall_C" (`KismetMathLibrary.Conv_VectorToTransform` (+ (* (`self.GetActorForwardVector` _returnvalue) (100.0 100.0 500.0)) (`self.K2_GetActorLocation` _returnvalue))) "Undefined" "MultiplyWithRoot" null null))

(fn `UserConstructionScript`)